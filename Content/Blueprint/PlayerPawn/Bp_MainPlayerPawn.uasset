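; Main player pawn that acts as a side-scrolling camera, with keyboard panning, screen-edge mouse panning and wheel zoom.
; BeginPlay adds the BaseInput Enhanced Input context, and AI_Move feeds movement input along the actor's right vector.
; Tick offsets the pawn along world X near the left or right viewport edge, without delta-time scaling.
; The legacy MouseWheelAxis event adjusts spring arm length within clamped limits.
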(event Input|EnhancedActionEvents|EnhancedInputActionAI_Move
  (params (ActionValue :type Vector%202D%20Structure) (ElapsedSeconds :type Float%20%28double-precision%29) (TriggeredSeconds :type Float%20%28double-precision%29) (InputAction :type Input%20Action%20Object%20Reference :default "/Game/Blueprint/PlayerPawn/AI_Move.AI_Move"))
  ;[0.15 0.15 0.15 0.5] a\d camera movement
  (Pawn|Input|AddMovementInput (Transformation|GetActorRightVector) (.y ActionValue) false))

(event EventBeginPlay
  ;[0.15 0.15 0.15 0.5] Add Mapping
  (Input|AddMappingContext (PlayerController|LocalPlayerSubsystems|GetEnhancedInputLocalPlayerSubsystem (Game|GetPlayerController 0)) "/Game/Blueprint/PlayerPawn/BaseInput.BaseInput" 0 "(bIgnoreAllPressedKeysUntilRelease=True,bForceImmediately=False,bNotifyUserSettings=False)"))

(event Collision|EventActorBeginOverlap
  (params (OtherActor :type Actor%20Object%20Reference)))

(event EventTick
  (params (DeltaSeconds :type Float%20%28single-precision%29))
  (Utilities|FlowControl|Sequence
    (:then_0
      ;[0.15 0.15 0.15 0.5] Move camera left Mouse
      (if (< (.LocationX (Game|Player|GetMousePosition (Game|GetPlayerController 0))) (Variables|Default|GetEdgeThreshold))
        (Transformation|AddActorWorldOffset (Math|Vector|MakeVector (Variables|Default|GetCameraSpeed) 0.0 0.0))))
    (:then_1
      ;[0.15 0.15 0.15 0.5] Move camera right
      (if (> (.LocationX (Game|Player|GetMousePosition (Game|GetPlayerController 0))) (- (.x (Viewport|GetViewportSize)) (Variables|Default|GetEdgeThreshold)))
        (Transformation|AddActorWorldOffset (Math|Vector|MakeVector (* (Variables|Default|GetCameraSpeed) -1.0) 0.0 0.0))))))

(event Input|MouseEvents|MouseWheelAxis
  (params (AxisValue :type Float%20%28single-precision%29))
  ;[0.15 0.15 0.15 0.5] Zoom
  (Variables|/Script/Engine.SpringArmComponent|SetTargetArmLength (Variables|Default|GetCameraSpringArm) (Math|Float|Clamp(Float) (- (Variables|/Script/Engine.SpringArmComponent|GetTargetArmLength (Variables|Default|GetCameraSpringArm)) (* AxisValue (Variables|Default|GetZoomSpeed))) 3e+01 1e+03)))

(fn ConstructionScript)