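; BP_GameManager is a game manager Blueprint that sets up the main UI and a toggleable build menu.
; On BeginPlay it shows the mouse cursor and adds a WB_UI widget to the viewport.
; The B key flips ShowBuildMenu, either creating a WB_Store widget or removing the one referenced by ShowWidget.
; The newly created store widget is not assigned to ShowWidget in this graph.
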(event EventBeginPlay
  ;[0.15 0.15 0.15 0.5] Show Cursor
  (Variables|/Script/Engine.PlayerController|SetbShowMouseCursor (Game|GetPlayerController 0) true)
  (bind _returnvalue (UserInterface|CreateWidget "/Game/Maps/Menu/WB_UI.WB_UI_C"))
  (UserInterface|Viewport|AddtoViewport _returnvalue 0))

(event Input|KeyboardEvents|B
  (params (Key :type Key%20Structure :default "None"))
  ;[0.15 0.15 0.15 0.5] Show\HideBuild Menu
  (:Pressed
    (if (Variables|Default|GetShow%20Build%20Menu)
      (Widget|RemovefromParent (Variables|Default|GetShowWidget))
      (Variables|Default|SetShow%20Build%20Menu false)
      (else
        (bind _returnvalue (UserInterface|CreateWidget "/Game/Maps/Menu/WB_Store.WB_Store_C"))
        (UserInterface|Viewport|AddtoViewport _returnvalue 0)
        (Variables|Default|SetShow%20Build%20Menu true)))))

(fn ConstructionScript)