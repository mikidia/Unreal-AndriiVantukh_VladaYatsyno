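; Guest spawn manager Blueprint meant to create a Bp_Guest widget with a random texture at a random spawn point.
; BeginPlay calls SpawnWidget and SwapTextures, but both events are empty, so nothing spawns.
; The disconnected logic creates the widget, positions it from a random "SpawnPoint" actor's location, and stores the "Lobby" actor.
; A second unconnected chain passes a random GuestTextures entry to the widget's GetIcon.
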(event Custom|SwapTextures)

(event Custom|SpawnWidget)

(event EventBeginPlay
  (CallFunction|SpawnWidget)
  (CallFunction|SwapTextures))

(fn ConstructionScript)