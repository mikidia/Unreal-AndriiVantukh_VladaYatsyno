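; Guest spawn manager that places one randomly styled guest sprite in the level when play begins.
; On BeginPlay it gathers all actors tagged SpawnPoint and spawns a BP_SpriteActor at a random one's transform.
; It then sets that actor's Paper2D sprite component to a random entry from the GuestSprites array.
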(event EventBeginPlay
  (bind _outactors (Actor|GetAllActorswithTag "SpawnPoint"))
  (bind _output_get (Variables|Default|SetSpawnPointsArray _outactors))
  (bind _returnvalue (Game|SpawnActorfromClass "/Game/Collections/Girl_1/BP_SpriteActor.BP_SpriteActor_C" (Transformation|GetActorTransform (Utilities|Array|Get(acopy) (Variables|Default|GetSpawnPointsArray) (Math|Random|RandomIntegerinRange 0 (- (Utilities|Array|Length _output_get) 1)))) "Undefined" "MultiplyWithRoot" 0 0))
  (Rendering|Components|Sprite|SetSprite (Actor|GetComponentbyClass _returnvalue "/Script/Paper2D.PaperSpriteComponent") (Utilities|Array|Get(acopy) (Variables|Default|GetGuestSprites) (Math|Random|RandomIntegerinRange 0 (- (Utilities|Array|Length (Variables|Default|GetGuestSprites)) 1)))))

(fn ConstructionScript)