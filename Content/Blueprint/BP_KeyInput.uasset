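; BP_KeyInput handles the pause key and holds helpers for saving game data.
; The AI_Pause input action creates the PauseMenu widget once, then toggles it in the viewport along with game pause and input mode.
; Load reads the "2DMap" slot into a BP_SaveGame, or creates and saves a new one if none exists; Save writes it back.
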(event Input|EnhancedActionEvents|EnhancedInputActionAI_Pause
  (params (ActionValue :type Boolean) (ElapsedSeconds :type Float%20%28double-precision%29) (TriggeredSeconds :type Float%20%28double-precision%29) (InputAction :type Input%20Action%20Object%20Reference :default "/Game/Input/AI_Pause.AI_Pause"))
  ;[0.15 0.15 0.15 0.5] Pause Game
  (:Started
    (Utilities|IsValid (Variables|Default|GetNewVar)
      (:Is%20Valid
        _)
      (:Is%20Not%20Valid
        (bind _returnvalue (UserInterface|CreateWidget "/Game/Maps/Menu/PauseMenu.PauseMenu_C"))
        (Variables|Default|SetNewVar _returnvalue)))
    (if (Game|IsGamePaused)
      (Widget|RemovefromParent (Variables|Default|GetNewVar))
      (Game|SetGamePaused false)
      (Input|SetInputModeGameOnly (Game|GetPlayerController 0) false)
      (else
        (UserInterface|Viewport|AddtoViewport (Variables|Default|GetNewVar) 0)
        (Game|SetGamePaused true)
        (Input|SetInputModeGameandUI (Game|GetPlayerController 0) (Variables|Default|GetNewVar) "DoNotLock" true false)))))

(fn Load
  ;[0.15 0.15 0.15 0.5] Savings
  (bind _returnvalue (SaveGame|DoesSaveGameExist "2DMap"))
  (if _returnvalue
    (bind _returnvalue_2 (SaveGame|LoadGamefromSlot "2DMap"))
    (bind _asbp_save_game (Utilities|Casting|CastToBP_SaveGame _returnvalue_2))
    (Variables|Default|SetSaveGame _asbp_save_game)
    (else
      (bind _returnvalue_3 (SaveGame|CreateSaveGameObject "/Game/Blueprint/BP_SaveGame.BP_SaveGame_C"))
      (Variables|Default|SetSaveGame _returnvalue_3)
      (CallFunction|Save))))

(fn Save
  (SaveGame|SaveGametoSlot (Variables|Default|GetSaveGame) "2DMap"))