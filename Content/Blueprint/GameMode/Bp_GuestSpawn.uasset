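; Bp_GuestSpawn is a spawner that keeps the level topped up with BP_Guest actors.
; Every tick it counts all BP_Guest actors in the world and calls Spawn while the count is below MaxGuest, adding at most one guest per frame.
; Spawn places a guest at the location of a random actor tagged SpawnPoint, with a fixed rotation and scale.
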(event EventTick
  (params (DeltaSeconds :type Float%20%28single-precision%29))
  (bind _outactors (Actor|GetAllActorsOfClass "/Game/Maps/Actors/BP_Guest.BP_Guest_C"))
  (if (< (Utilities|Array|Length _outactors) (Variables|Default|GetMaxGuest))
    (CallFunction|Spawn)))

(fn ConstructionScript)

(fn Spawn
  (bind _outactors (Actor|GetAllActorswithTag "SpawnPoint"))
  (Game|SpawnActorfromClass "/Game/Maps/Actors/BP_Guest.BP_Guest_C" (Math|Transform|MakeTransform (.location (Transformation|GetActorTransform (.OutItem (Utilities|Array|Random _outactors)))) "0.000000,-90.000000,0.000000" "3.000000,3.000000,3.000000") "Undefined" "MultiplyWithRoot" 0 0))