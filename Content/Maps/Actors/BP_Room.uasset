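; BP_Room is a room actor that tracks whether it is free and can award money through the UI.
; It hides its progress bar widget and marks itself free on BeginPlay.
; CdRoom claims a free room, shows the bar and calls the still-empty Percent stub, or returns true if already occupied.
; AddMoney finds top-level WB_UI widgets and adds a fixed amount through them.
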(event Custom|AddMoney
  (bind _foundwidgets (Widget|GetAllWidgetsOfClass "/Game/Maps/Menu/WB_UI.WB_UI_C" true))
  (Default|AddMoney _foundwidgets 1e+02))

(event EventBeginPlay
  (CallFunction|HideWidget))

(event Collision|EventActorBeginOverlap
  (params (OtherActor :type Actor%20Object%20Reference)))

(event EventTick
  (params (DeltaSeconds :type Float%20%28single-precision%29)))

(fn ConstructionScript)

(fn CdRoom
  (if (Variables|Default|GetIsFree)
    (Variables|Default|SetIsFree false)
    (Widget|SetVisibility (UserInterface|GetWidget (Variables|Default|GetProgressBarWidget)) "Visible")
    (CallFunction|Percent)
    (else
      (return true))))

(fn Percent
  (if (Variables|Default|GetIsFree)
    _))

(fn HideWidget
  (Widget|SetVisibility (UserInterface|GetWidget (Variables|Default|GetProgressBarWidget)) "Hidden")
  (Variables|Default|SetIsFree true))