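; Guest actor that the player picks up with a click and carries under the cursor to place in a BP_Room.
; While dragged, Tick moves it on a fixed-Y plane using mouse delta, start position and camera location.
; A second click line-traces from the cursor and calls CdRoom on a hit room, destroying the guest on success or calling BackToStartPoint otherwise.
; The drag flag is never cleared.
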(event EventBeginPlay)

(event Collision|EventActorBeginOverlap
  (params (OtherActor :type Actor%20Object%20Reference)))

(event EventTick
  (params (DeltaSeconds :type Float%20%28single-precision%29))
  (bind _returnvalue (Game|GetPlayerCameraManager 0))
  (bind _returnvalue_2 (Game|GetPlayerController 0))
  (bind _startmousepos (Variables|Default|GetStartMousePos))
  (bind _startpos (Variables|Default|GetStartPos))
  (bind (_locationx _locationy) (Game|Player|GetMousePosition _returnvalue_2))
  (bind _returnvalue_3 (Camera|GetCameraLocation _returnvalue))
  (if (Variables|Default|GetIsDragged)
    (Transformation|SetActorLocation self (Math|Vector|MakeVector (+ (- (.x _startmousepos) _locationx) (.x _startpos) (.x _returnvalue_3)) 219.0 (+ (- (.y _startmousepos) _locationy) (.y _startpos) (.z _returnvalue_3))) false false)))

(event MouseInput|EventActorOnClicked
  (params (ButtonPressed :type Key%20Structure :default "None"))
  (bind _returnvalue (Game|GetPlayerController 0))
  (bind _returnvalue_2 (Game|GetPlayerController 0))
  (bind _self self)
  (bind _returnvalue_3 (Transformation|GetActorLocation _self))
  (bind (_worldlocation _worlddirection) (Game|Player|ConvertMouseLocationToWorldSpace _returnvalue))
  (bind (_locationx _locationy) (Game|Player|GetMousePosition _returnvalue_2))
  (if (Variables|Default|GetIsDragged)
    (bind _outhit (Collision|LineTraceByChannel _worldlocation (+ _worldlocation (* "1000.000000,1000.000000,1000.000000" _worlddirection)) "TraceTypeQuery1" false 0 "None"))
    (bind _asbp_room (Utilities|Casting|CastToBP_Room (.hitactor _outhit)))
    (bind _isfree (Default|CdRoom _asbp_room))
    (if _isfree
      (Actor|DestroyActor)
      (else
        (CallFunction|BacktoStartPoint)))
    (else
      (Variables|Default|SetIsDragged true)
      (Variables|Default|SetStartPos (Math|Vector2D|MakeVector2D (.x _returnvalue_3) (.z _returnvalue_3)))
      (Variables|Default|SetStartMousePos (Math|Vector2D|MakeVector2D _locationx _locationy)))))

(fn ConstructionScript)

(fn BacktoStartPoint
  (bind _startpos (Variables|Default|GetStartPos))
  (Transformation|SetActorLocation self (Math|Vector|MakeVector (.x _startpos) 219.0 (.y _startpos)) false false))