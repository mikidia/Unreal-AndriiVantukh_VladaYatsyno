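; BP_Guest is a guest actor that the player picks up by clicking, after which it follows the mouse.
; Clicking sets a drag flag and stores the actor's X/Z position and the cursor's screen position.
; While dragging, Tick adds the start-minus-current cursor offset, in raw pixels, to the stored X/Z, leaving Y at zero.
; Nothing in this Blueprint clears the drag flag.
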(event EventBeginPlay)

(event Collision|EventActorBeginOverlap
  (params (OtherActor :type Actor%20Object%20Reference)))

(event EventTick
  (params (DeltaSeconds :type Float%20%28single-precision%29))
  (bind _returnvalue (Game|GetPlayerController 0))
  (bind _startmousepos (Variables|Default|GetStartMousePos))
  (bind _startpos (Variables|Default|GetStartPos))
  (bind (_locationx _locationy) (Game|Player|GetMousePosition _returnvalue))
  (if (Variables|Default|GetIsDragged)
    (Transformation|SetActorLocation self (Math|Vector|MakeVector (+ (- (.x _startmousepos) _locationx) (.x _startpos)) 0.0 (+ (- (.y _startmousepos) _locationy) (.y _startpos))) false false)))

(event MouseInput|EventActorOnClicked
  (params (ButtonPressed :type Key%20Structure :default "None"))
  (bind _returnvalue (Game|GetPlayerController 0))
  (bind _self self)
  (bind _returnvalue_2 (Transformation|GetActorLocation _self))
  (bind (_locationx _locationy) (Game|Player|GetMousePosition _returnvalue))
  (Variables|Default|SetIsDragged true)
  (Variables|Default|SetStartPos (Math|Vector2D|MakeVector2D (.x _returnvalue_2) (.z _returnvalue_2)))
  (Variables|Default|SetStartMousePos (Math|Vector2D|MakeVector2D _locationx _locationy)))

(fn ConstructionScript)